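; WidgetControl_Class is an input relay Blueprint that drives a menu widget from input actions.
; Menu Up and Menu Down presses call ChangeMenuSelect on the MenuWIdgetRef variable to step the selection backward or forward.
; Menu Select calls SelectMenu, and Menu OpenClose only calls CloseMenu, so this Blueprint never opens the menu itself.
; The graph does not assign the widget reference or check its validity, and the construction script is empty.
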(event Input|ActionEvents|InputActionMenuUp
  (params (Key :type Key%20Structure))
  ;[1 1 1] 入力に対する処理(Up, Down, Select)
  (:Pressed
    (Default|ChangeMenuSelect (Variables|Default|GetMenu%20WIdget%20Ref) -1)))

(event Input|ActionEvents|InputActionMenuDown
  (params (Key :type Key%20Structure))
  ;[1 1 1] 入力に対する処理(Up, Down, Select)
  (:Pressed
    (Default|ChangeMenuSelect (Variables|Default|GetMenu%20WIdget%20Ref) 1)))

(event Input|ActionEvents|InputActionMenuSelect
  (params (Key :type Key%20Structure))
  ;[1 1 1] 入力に対する処理(Up, Down, Select)
  (:Pressed
    (Default|SelectMenu (Variables|Default|GetMenu%20WIdget%20Ref))))

(event Input|ActionEvents|InputActionMenuOpenClose
  (params (Key :type Key%20Structure))
  ;[1 1 1] 入力に対する処理(Up, Down, Select)
  (:Pressed
    (Default|CloseMenu (Variables|Default|GetMenu%20WIdget%20Ref))))

(fn ConstructionScript)