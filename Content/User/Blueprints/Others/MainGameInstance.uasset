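; Game instance that holds shared UI widgets and stage state for a stage-based game with gravity objects and fuel scoring.
; Init creates the menu, HUD, result and fade widgets, which helper functions use for fading and results.
; Stage switches clamp the index and reopen a scene by name; reloads first save the player's movement trace.
; It also caches gravity-interface actors and serves per-stage data, though GetCurrentMaxFuel returns StageSize.
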(event EventInit
  ;[1 1 1] Game Instanceの変数にオブジェクトの参照を格納する
  (Utilities|FlowControl|Sequence
    (:then_0
      (bind _returnvalue (UserInterface|CreateWidget "/Game/User/Blueprints/Widget/GameClear_Widget.GameClear_Widget_C" (Game|GetPlayerController 0)))
      (Variables|Default|SetGameClear%20Widget%20Ref _returnvalue))
    (:then_1
      (bind _returnvalue_2 (UserInterface|CreateWidget "/Game/User/Blueprints/Widget/GameOver_Widget.GameOver_Widget_C" (Game|GetPlayerController 0)))
      (Variables|Default|SetGameOver%20Widget%20Ref _returnvalue_2))
    (:then_2
      (bind _returnvalue_3 (UserInterface|CreateWidget "/Game/User/Blueprints/Widget/PauseMenu_Widget.PauseMenu_Widget_C" (Game|GetPlayerController 0)))
      (Variables|Default|SetPause%20Menu%20Widget%20Ref _returnvalue_3))
    (:then_3
      (bind _returnvalue_4 (UserInterface|CreateWidget "/Game/User/Blueprints/Widget/FadingWidget.FadingWidget_C" (Game|GetPlayerController 0)))
      (Variables|Default|SetFading%20Widget%20Ref _returnvalue_4))
    (:then_4
      (bind _returnvalue_5 (UserInterface|CreateWidget "/Game/User/Blueprints/Widget/Result_Widget.Result_Widget_C" (Game|GetPlayerController 0)))
      (Variables|Default|SetResult%20Widget%20Ref _returnvalue_5))
    (:then_5
      (bind _returnvalue_6 (UserInterface|CreateWidget "/Game/User/Blueprints/Widget/MainUI_Widget.MainUI_Widget_C" (Game|GetPlayerController 0)))
      (Variables|Default|SetMainUI%20Widget%20Ref _returnvalue_6))))

(fn GetCurrentStageName
  (return (Utilities|Array|Get(acopy) (Variables|Default|GetStage%20Name%20List) (Variables|Default|GetStage%20Select%20Index))))

(fn ChangeStageDiff
  (params (Select%20Index%20Diff :type Integer))
  ;[1 1 1] StageをSelect Index Diffの値分だけ変更し、ステージを切り替える
  (Stage|ChangeStageDirect (+ Select%20Index%20Diff (Variables|Default|GetStage%20Select%20Index))))

(fn ChangeStageDirect
  (params (Change%20Stage%20Index :type Integer))
  ;[1 1 1] StageをChange Stage Indexの値に変更し、ステージを切り替える
  (Variables|Default|SetStage%20Select%20Index Change%20Stage%20Index)
  (Stage|AdjustStageSelectIndex)
  (Utilities|Array|Clear (Variables|Default|GetRecent%20Trace%20Record%20Data))
  (Game|OpenLevel(byName) (Get|GetSceneName "NewEnumerator2")))

(fn AdjustStageSelectIndex
  ;[1 1 1] Stage Select Indexを適正な値に調整する
  (Variables|Default|SetStage%20Select%20Index (Math|Integer|Max(Integer) (Variables|Default|GetStage%20Select%20Index)))
  (Variables|Default|SetStage%20Select%20Index (Math|Integer|Min(Integer) (Variables|Default|GetStage%20Select%20Index) (- (Utilities|Array|Length (Variables|Default|GetStage%20Name%20List)) 1))))

(fn ReloadCurrentStage
  (Utilities|FlowControl|Sequence
    (:then_0
      ;[1 1 1] 今回のプレイヤーの移動記録情報を格納する
      (Utilities|Array|Clear (Variables|Default|GetRecent%20Trace%20Record%20Data))
      (Variables|Default|SetRecent%20Trace%20Record%20Data (Variables|/Game/User/Blueprints/Class/PlayerObject_Class.PlayerObject_Class_C|GetTrace%20Record%20Data (Variables|Default|GetPlayer%20Object%20Ref))))
    (:then_1
      ;[1 1 1] MainMapを再読み込みする
      (Game|OpenLevel(byName) (Get|GetSceneName "NewEnumerator2")))))

(fn GetSceneName
  (params (Scene :type SceneName_Enum%20Enum :default "NewEnumerator0"))
  (return (Utilities|Array|Get(acopy) (Variables|Default|GetScene%20Name%20List) (Math|Conversions|ToInteger(Byte) Scene))))

(fn Fading
  (params (Flag%20Pause :type Boolean) (Fading%20Color :type Linear%20Color%20Structure) (Fade%20Select :type EUMGSequencePlayMode%20Enum :default "Forward") (Fading%20Time :type Float%20%28single-precision%29))
  ;[1 1 1] ウィジェットを呼び出してフェーディング処理を行う
  (UserInterface|Viewport|AddtoViewport (Variables|Default|GetFading%20Widget%20Ref) 0)
  (Game|SetGamePaused Flag%20Pause)
  (Default|Fading (Variables|Default|GetFading%20Widget%20Ref) Fading%20Color Fade%20Select Fading%20Time))

(fn DispatchFadeEndEvent
  (params (イベント :type Delegate%20%28by%20ref%29))
  ;[1 1 1] フェーディング終了時のイベントを設定する
  (EventDispatchers|BindEventtoFadingFinish (Variables|Default|GetFading%20Widget%20Ref) イベント))

(fn GetCurrentStageSize
  ;[1 1 1] 各ステージの半径を取得する
  (return (.stagesize (Utilities|Array|Get(acopy) (Variables|Default|GetStageDataList) (Variables|Default|GetStage%20Select%20Index)))))

(fn ReadGravityObject
  ;[1 1 1] ステージ上の重力を持ったアクターを取得し、リストに格納する
  (Utilities|Array|Clear (Variables|Default|GetGravity%20Object%20List))
  (bind _outactors (Actor|GetAllActorswithInterface "/Game/User/Blueprints/Interface/GravityEffect_Interface.GravityEffect_Interface_C"))
  (bind _output_get (Variables|Default|SetGravity%20Object%20List _outactors))
  (for _array_element _output_get
    _))

(fn ShowGameResult
  (params (Item%20Cnt :type Integer) (Fuel%20Value :type Float%20%28single-precision%29))
  (Widget|RemovefromParent (Variables|Default|GetMainUI%20Widget%20Ref))
  (Default|ShowMenu (Variables|Default|GetResult%20Widget%20Ref) true)
  (Default|SetResultValue (Variables|Default|GetResult%20Widget%20Ref) Item%20Cnt 0 Fuel%20Value (Get|GetCurrentMaxFuel) (Variables|/Game/User/Blueprints/Widget/MainUI_Widget.MainUI_Widget_C|GetSpend%20Time (Variables|Default|GetMainUI%20Widget%20Ref)))
  (Default|CalcMaxScore (Variables|Default|GetResult%20Widget%20Ref)))

(fn GetCurrentStageData
  (return (Utilities|Array|Get(acopy) (Variables|Default|GetStageDataList) (Variables|Default|GetStage%20Select%20Index))))

(fn GetCurrentMaxFuel
  ;[1 1 1] 各ステージの半径を取得する
  (return (.stagesize (Utilities|Array|Get(acopy) (Variables|Default|GetStageDataList) (Variables|Default|GetStage%20Select%20Index)))))

(fn GetBestTraceRecoedList
  (return (.bestscoretracerecord (Utilities|Array|Get(acopy) (Variables|Default|GetStageDataList) (Variables|Default|GetStage%20Select%20Index)))))