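; Movement component that moves its owner in 2D (X/Y) under the gravity of planets and other objects in the GameInstance's gravity list.
; Each enabled tick sums their mass- and position-based pulls, integrates velocity and position, and clamps speed, zeroing it when nearly stopped.
; While the promotion flag is set by an added boost, the owner's yaw follows its velocity.
; Exposed functions add boosts, rotate velocity, set max speed and toggle updates.
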(event EventBeginPlay
  ;[1 1 1] Game Instanceを変数に格納する
  (bind _asmain_game_instance (Utilities|Casting|CastToMainGameInstance (Game|GetGameInstance)))
  (Variables|Default|SetGame%20Instance%20Ref _asmain_game_instance))

(event EventTick
  (params (DeltaSeconds :type Float%20%28single-precision%29))
  ;[1 1 1] 重力計算を行う
  (if (CallFunction|CheckTickEnable)
    (CallFunction|UpdateGravityEffect)
    (CallFunction|UpdateSpeed)
    (CallFunction|UpdatePosition)
    (CallFunction|UpdateRotation)))

(fn UpdateGravityEffect
  ;[1 1 1] 各惑星の重力効果を取得し、Gravity Effect 変数に格納する
  (Variables|Default|SetGravity%20Effect "")
  (for _array_element (Variables|/Game/User/Blueprints/Others/MainGameInstance.MainGameInstance_C|GetGravity%20Object%20List (Variables|Default|GetGame%20Instance%20Ref))
    (Utilities|IsValid _array_element
      (:Is%20Valid
        (CallFunction|CalcGravityEffect _array_element))))
  (return))

(fn CalcGravityEffect
  (params (Actor%20Ref :type Actor%20Object%20Reference))
  (bind _returnvalue (Components|GetOwner))
  ;[1 1 1] Planet BP Ref より得られる重力効果データを Gravity Effect に格納する
  (bind _mass_value (Class|PhisycalInterface|GetMassValue(Message) _returnvalue))
  (bind _gravity_effect (Class|GravityEffectInterface|GetGravityEffect(Message) Actor%20Ref _mass_value (Math|Conversions|ToVector2D(Vector) (Transformation|GetActorLocation _returnvalue))))
  (Variables|Default|SetGravity%20Effect (+ _gravity_effect (Variables|Default|GetGravity%20Effect))))

(fn UpdateSpeed
  ;[1 1 1] 重力による速度計算
  (Variables|Default|SetMove%20Speed (+ (Variables|Default|GetMove%20Speed) (* (Variables|Default|GetGravity%20Effect) (Utilities|Time|GetWorldDeltaSeconds))))
  (CallFunction|AdjustSpeedValue))

(fn UpdatePosition
  ;[1 1 1] 重力による位置情報更新処理
  (Transformation|AddActorWorldOffset (Components|GetOwner) (Math|Conversions|ToVector(Vector2D) (* (Variables|Default|GetMove%20Speed) (Utilities|Time|GetWorldDeltaSeconds)))))

(fn CheckTickEnable
  ;[1 1 1] アップデートを行うかどうかをチェックする
  (return (and (Variables|Default|GetFlag%20Update) (Class|Actor|IsActorTickEnabled (Components|GetOwner)))))

(fn UpdateRotation
  ;[1 1 1] 移動方向に合わせてプレイヤーの回転処理を行う
  (if (Variables|Default|GetFlag%20Promotion)
    (Transformation|SetActorRotation (Components|GetOwner) (Math|Rotator|MakeRotator 0.0 0.0 (+ (.yaw (Math|Rotator|MakeRotfromZ (Math|Conversions|ToVector(Vector2D) (Variables|Default|GetMove%20Speed)))) 1.8e+02)))))

(fn AdjustSpeedValue
  ;[1 1 1] 速度補正(速度が０以下もしくはMax Speed以上の時に補正する)
  (bind _output_get (LocalVariables|SetSpeed%20Value (Math|Vector2D|Vector2DLength (Variables|Default|GetMove%20Speed))))
  (LocalVariables|SetSpeed%20Value (Math|Float|Max(Float) _output_get 0.0))
  (LocalVariables|SetSpeed%20Value (Math|Float|Min(Float) (LocalVariables|GetSpeed%20Value) (Variables|Default|GetMax%20Speed%20Value)))
  (if (Math|Float|NearlyEqual(Float) (LocalVariables|GetSpeed%20Value) 0.0 1e+01)
    (LocalVariables|SetSpeed%20Value 0.0)
    (Variables|Default|SetFlag%20Promotion false))
  (Variables|Default|SetMove%20Speed (* (Math|Vector2D|Normalize2D (Variables|Default|GetMove%20Speed)) (LocalVariables|GetSpeed%20Value))))

(fn AddActorPromotion
  (params (Actor%20Acc :type Vector%202D%20Structure))
  (Variables|Default|SetMove%20Speed (+ Actor%20Acc (Variables|Default|GetMove%20Speed)))
  (Variables|Default|SetFlag%20Promotion true))

(fn CheckCanBlaking
  (return (Variables|Default|GetFlag%20Promotion)))

(fn SetUpdateFlag
  (params (Flag :type Boolean))
  (Variables|Default|SetFlag%20Update Flag))

(fn SetMaxSpeed
  (params (Max%20Speed :type Float%20%28single-precision%29))
  (Variables|Default|SetMax%20Speed%20Value Max%20Speed))

(fn AddRotate
  (params (RotZ :type Float%20%28single-precision%29))
  (Variables|Default|SetMove%20Speed (Math|Conversions|ToVector2D(Vector) (Math|Vector|RotateVector (Math|Conversions|ToVector(Vector2D) (Variables|Default|GetMove%20Speed)) (Math|Rotator|MakeRotator 0.0 0.0 RotZ)))))