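; Player actor for a slingshot-style gravity game, launched by dragging the mouse or gamepad stick and steered past planets.
; While pressed, Tick derives direction and speed from the pull; otherwise it sums planet gravity, updates velocity and moves the actor manually.
; A CheckPush gate-and-delay macro repeats fuel-consuming boost or brake while held.
; Overlap gameplay tags trigger reset, game-over or clear menus; SetStageData caches planets and start position.
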(event EventBeginPlay
  ;[1 1 1] Game Instanceを変数に格納する
  (bind _asmain_game_instance (Utilities|Casting|CastToMainGameInstance (Game|GetGameInstance)))
  (Variables|Default|SetGame%20Instance%20Ref _asmain_game_instance))

(event EventTick
  (params (DeltaSeconds :type Float%20%28single-precision%29))
  (if (Variables|Default|GetFlag%20Press)
    ;[1 1 1] 引っ張り状況から射出方向と速度を算出して格納する
    (bind _returnvalue (Class|WidgetLayoutLibrary|GetMousePositiononViewport))
    (Variables|Default|SetSpeed%20Direction (Math|Vector2D|MakeVector2D (.y (Math|Vector2D|Normalize2D (+ (* (Variables|Default|GetPad%20Stick%20Point) (Variables|Default|GetPadStick2Speed%20Value)) (- _returnvalue (Variables|Default|GetPull%20Start%20Point))))) (* (.x (Math|Vector2D|Normalize2D (+ (* (Variables|Default|GetPad%20Stick%20Point) (Variables|Default|GetPadStick2Speed%20Value)) (- _returnvalue (Variables|Default|GetPull%20Start%20Point))))) -1.0)))
    (Variables|デフォルト|SetSpeed%20Value (/ (Math|Vector2D|Vector2DLength (+ (* (Variables|Default|GetPad%20Stick%20Point) (Variables|Default|GetPadStick2Speed%20Value)) (- _returnvalue (Variables|Default|GetPull%20Start%20Point)))) (Variables|Default|GetMouse2Speed%20Value)))
    (Development|PrintString (Utilities|String|Append "Speed Value : " (Utilities|String|ToString(Float) (Variables|デフォルト|GetSpeed%20Value))))
    (Development|PrintString (Utilities|String|Append "Speed Direction : " (Utilities|String|ToString(Vector2d) (Variables|Default|GetSpeed%20Direction))))
    (else
      ;[1 1 1] 移動処理系(重力処理→位置更新処理→減速処理→速度規格化処理)
      (CallFunction|SetGravityEffect)
      (CallFunction|UpdateSpeed)
      (CallFunction|UpdatePosition))))

(event Collision|EventActorBeginOverlap
  (params (OtherActor :type Actor%20Object%20Reference))
  ;[1 1 1] 接触判定(Tag : Stop → 速度を0にする、Tag : End → ゲームを停止する)
  (CallFunction|ApplyCollisionEffect OtherActor))

(event Input|ActionEvents|InputActionResetGame
  (params (Key :type Key%20Structure))
  ;[1 1 1] 初期状態に戻す
  (:Pressed
    (CallFunction|ResetPlayer)))

(event Input|ActionEvents|InputActionSpeedUp
  (params (Key :type Key%20Structure))
  ;[1 1 1] 加速処理(LShift)
  (:Pressed
    (Utilities|CheckPush 0.1 :!label _label
      (:Main%20Action
        (CallFunction|ChangeSpeedbyBoost (Variables|Default|GetBoost%20Forward%20Value)))
      (:Finalize%20Action
        (Variables|Default|SetBoost%20Value 0.0))))
  (:Released
    (goto _label Released)))

(event Input|ActionEvents|InputActionSpeedDown
  (params (Key :type Key%20Structure))
  ;[1 1 1] 減速処理(スペースバー)
  (:Pressed
    (Utilities|CheckPush 0.1 :!label _label
      (:Main%20Action
        (CallFunction|ChangeSpeedbyBoost (* (Variables|Default|GetBoost%20Back%20Value) -1.0)))
      (:Finalize%20Action
        (Variables|Default|SetBoost%20Value 0.0))))
  (:Released
    (goto _label Released)))

(event Input|ActionEvents|InputActionLanchTrigger
  (params (Key :type Key%20Structure))
  ;[1 1 1] 射出処理(マウスクリックで引っ張ってマウスリリースで発射)
  (:Pressed
    (if (== (Variables|デフォルト|GetSpeed%20Value) 0.0)
      (Variables|Default|SetFlag%20Press true)
      (bind _returnvalue (Class|WidgetLayoutLibrary|GetMousePositiononViewport))
      (Variables|Default|SetPull%20Start%20Point _returnvalue)))
  (:Released
    (Variables|Default|SetFlag%20Press false)))

(event Input|GamepadEvents|GamepadLeftX
  (params (AxisValue :type Float%20%28single-precision%29))
  ;[1 1 1] Padによる射出処理
  (if (Variables|Default|GetFlag%20Press)
    (Variables|Default|SetPad%20Stick%20Point (Math|Vector2D|MakeVector2D AxisValue (.y (Variables|Default|GetPad%20Stick%20Point))))))

(event Input|GamepadEvents|GamepadLeftY
  (params (AxisValue :type Float%20%28single-precision%29))
  ;[1 1 1] Padによる射出処理
  (if (Variables|Default|GetFlag%20Press)
    (bind _output_get (Variables|Default|SetPad%20Stick%20Point (Math|Vector2D|MakeVector2D (.x (Variables|Default|GetPad%20Stick%20Point)) (* AxisValue -1.0))))
    (Development|PrintString (Utilities|String|ToString(Vector2d) _output_get))))

(fn ConstructionScript)

(fn AdjustSpeedValue
  (bind _max_speed_value (Variables|Default|GetMax%20Speed%20Value))
  ;[1 1 1] 速度補正(速度が０以下もしくはMax Speed以上の時に補正する)
  (if (< (Variables|デフォルト|GetSpeed%20Value) 0.0)
    (Variables|デフォルト|SetSpeed%20Value 0.0)
    (elif (> (Variables|デフォルト|GetSpeed%20Value) _max_speed_value)
      (Variables|デフォルト|SetSpeed%20Value _max_speed_value))))

(fn ChangeSpeedbyBoost
  (params (Change%20Speed%20Value :type Float%20%28single-precision%29))
  ;[1 1 1] Change Speed Value(+なら加速、-なら減速) の値に応じて Speed Value の値を変更する
  (if (Math|Boolean|ANDBoolean (> (Variables|Default|GetFuel%20Value) 0.0) (> (Variables|デフォルト|GetSpeed%20Value) 0.0) (< (Variables|デフォルト|GetSpeed%20Value) (Variables|Default|GetMax%20Speed%20Value)))
    (Variables|Default|SetBoost%20Value Change%20Speed%20Value)
    (Variables|Default|SetFuel%20Value (- (Variables|Default|GetFuel%20Value) (Variables|Default|GetSpending%20Fuel%20Value)))))

(fn ApplyCollisionEffect
  (params (Collided%20Actor :type Actor%20Object%20Reference))
  ;[1 1 1] 衝突したアクターのタグに応じて衝突処理を行う
  (bind _own_gameplay_tagcontainer (Class|CollisionTagInterface|GetCollisionTagContainer(Message) Collided%20Actor))
  (|SwitchGameplayTagContainer _own_gameplay_tagcontainer
    (:%28GameplayTags=%28%28TagName="Collision.Stop"%29%29%29
      (CallFunction|ResetPlayer))
    (:%28GameplayTags=%28%28TagName="Collision.End"%29%29%29
      (Default|ShowMenu (Variables|/Game/User/Blueprints/Class/MainGameInstance.MainGameInstance_C|GetGameOver%20Widget%20Ref (Variables|Default|GetGame%20Instance%20Ref))))
    (:%28GameplayTags=%28%28TagName="Collision.Clear"%29%29%29
      (Default|ShowMenu (Variables|/Game/User/Blueprints/Class/MainGameInstance.MainGameInstance_C|GetGameClear%20Widget%20Ref (Variables|Default|GetGame%20Instance%20Ref))))))

(fn SetGravityEffect
  ;[1 1 1] 各惑星の重力効果を取得し、Gravity Effect 変数に格納する
  (Variables|Default|SetGravity%20Effect "")
  (for _array_element (Variables|Default|GetPlanet%20List)
    (Utilities|IsValid _array_element
      (:Is%20Valid
        (CallFunction|StackGravityEffect _array_element))))
  (return))

(fn UpdatePosition
  ;[1 1 1] 現在の速度と重力効果をもとに位置情報を更新する
  (Transformation|AddActorWorldOffset (Math|Conversions|ToVector(Vector2D) (* (Variables|Default|GetSpeed%20Direction) (Variables|デフォルト|GetSpeed%20Value)) (Utilities|Time|GetWorldDeltaSeconds))))

(fn ResetPlayer
  ;[1 1 1] ゲームをリセットする(速度情報と位置情報を初期化する)
  (Transformation|SetActorLocation (Math|Conversions|ToVector(Vector2D) (Variables|Default|GetDefault%20Position)) false true)
  (Variables|デフォルト|SetSpeed%20Value 0.0)
  (Variables|Default|SetSpeed%20Direction "")
  (Variables|Default|SetBoost%20Value 0.0)
  (Variables|Default|SetGravity%20Effect "")
  (Variables|Default|SetFuel%20Value (Variables|Default|GetMax%20Fuel%20Value)))

(fn AddSpeedVector
  (params (Added%20Speed%20Vec :type Vector%202D%20Structure) (Flag%20Add :type Boolean))
  ;[1 1 1] プレイヤーの速度にAdded Speed Vecを加算する(Flag が false なら減算する)
  (Variables|Default|SetSpeed%20Direction (Math|Vector2D|Normalize2D (+ (* (* Added%20Speed%20Vec (Math|Float|SelectFloat -1.0 1.0 Flag%20Add)) (Utilities|Time|GetWorldDeltaSeconds)) (* (Variables|Default|GetSpeed%20Direction) (Variables|デフォルト|GetSpeed%20Value)))))
  (Variables|デフォルト|SetSpeed%20Value (Math|Vector2D|Vector2DLength (+ (* (* Added%20Speed%20Vec (Math|Float|SelectFloat -1.0 1.0 Flag%20Add)) (Utilities|Time|GetWorldDeltaSeconds)) (* (Variables|Default|GetSpeed%20Direction) (Variables|デフォルト|GetSpeed%20Value)))))
  (return))

(fn StackGravityEffect
  (params (Planet%20BP%20Ref :type Planet%20Class%20Object%20Reference))
  ;[1 1 1] Planet BP Ref より得られる重力効果データを Gravity Effect に格納する
  (bind _gravity_effect (Default|GetGravityEffect Planet%20BP%20Ref (Variables|Default|GetMass%20Value) (Math|Conversions|ToVector2D(Vector) (Transformation|GetActorLocation))))
  (Variables|Default|SetGravity%20Effect (+ _gravity_effect (Variables|Default|GetGravity%20Effect))))

(fn UpdateSpeed
  ;[1 1 1] ブースト効果と重力効果による速度の変更を処理する
  (Variables|デフォルト|SetSpeed%20Value (+ (Variables|デフォルト|GetSpeed%20Value) (* (Variables|Default|GetBoost%20Value) (Utilities|Time|GetWorldDeltaSeconds))))
  (CallFunction|AdjustSpeedValue)
  (CallFunction|AddSpeedVector (Variables|Default|GetGravity%20Effect) false))

(fn SetStageData
  ;[1 1 1] ステージ開始時にステージ情報を格納する
  (Variables|Default|SetDefault%20Position (Math|Conversions|ToVector2D(Vector) (Transformation|GetActorLocation)))
  (Utilities|Array|Clear (Variables|Default|GetPlanet%20List))
  (bind _outactors (Actor|GetAllActorsOfClass "/Game/User/Blueprints/Class/Planet_Class.Planet_Class_C"))
  (Variables|Default|SetPlanet%20List _outactors)
  (CallFunction|ResetPlayer))