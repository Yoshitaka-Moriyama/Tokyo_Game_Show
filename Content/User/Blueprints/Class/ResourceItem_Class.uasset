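; Base resource item actor that, once collected by overlapping the player, trails the player object in an ordered line.
; On overlap it checks gameplay tags, casts to PlayerObject_Class, then enables following and takes a follower number from the player.
; Each tick it snaps to a slot offset by that number, rotated with the yaw of the player reference held in MainGameInstance.
; Getters expose its gameplay tags and mass value.
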(event EventBeginPlay
  ;[1 1 1] Game Instanceを変数に格納する
  (bind _asmain_game_instance (Utilities|Casting|CastToMainGameInstance (Game|GetGameInstance)))
  (Variables|Default|SetGame%20Instance%20Ref _asmain_game_instance))

(event EventTick
  (params (DeltaSeconds :type Float%20%28single-precision%29))
  ;[1 1 1] 回収したプレイヤーに合わせて位置と回転角度を更新する
  (if (Variables|Default|GetFlag%20Follow)
    (CallFunction|SetRelativePosandRot)))

(event Collision|EventActorBeginOverlap
  (params (OtherActor :type Actor%20Object%20Reference))
  ;[1 1 1] あたり判定とPlayer Objの座標のセット
  (if (not (Variables|Default|GetFlag%20Follow))
    (CallFunction|CheckPlayerCollided OtherActor)))

(fn ConstructionScript)

(fn CheckPlayerCollided
  (params (Collided%20Actor :type Actor%20Object%20Reference))
  ;[1 1 1] 衝突したアクターがプレイヤーだった場合追従を開始する
  (bind _output_get (LocalVariables|SetTemp%20Actor Collided%20Actor))
  (bind _own_gameplay_tagcontainer (Class|GamePlayTagInterface|GetGamePlayTagContainer(Message) _output_get))
  (for _array_element (GameplayTags|BreakGameplayTagContainer _own_gameplay_tagcontainer)
    (|SwitchGameplayTag _array_element
      (:ObjectType.Player
        (bind _asplayer_object_class (Utilities|Casting|CastToPlayerObject_Class (LocalVariables|GetTemp%20Actor)))
        (Variables|Default|SetPlayer%20Object%20Class%20Ref _asplayer_object_class)
        (LocalVariables|SetTemp%20Frag true)
        (Utilities|FlowControl|Sequence
          (:then_0
            (Variables|Default|SetFlag%20Follow true))
          (:then_2
            (Variables|Default|SetFollower%20Number (Default|GetFollowerNumber (Variables|Default|GetPlayer%20Object%20Class%20Ref))))))))
  (return (LocalVariables|GetTemp%20Frag)))

(fn SetRelativePosandRot
  (bind _game_instance_ref (Variables|Default|GetGame%20Instance%20Ref))
  (bind _player_object_ref (Variables|/Game/User/Blueprints/Others/MainGameInstance.MainGameInstance_C|GetPlayer%20Object%20Ref _game_instance_ref))
  (bind _returnvalue (Transformation|GetActorRotation _player_object_ref))
  ;[1 1 1] オブジェクトの向きと位置をPlayerObjectに合わせて調整する
  (Transformation|SetActorRotation (Math|Rotator|MakeRotator 0.0 0.0 (+ (.yaw _returnvalue) 1.8e+02)))
  (Transformation|SetActorLocation (+ (Math|Vector|RotateVectorAroundAxis (Math|Vector|MakeVector (+ (* (Variables|Default|GetFollower%20Number) (Variables|Default|GetLength%20Between%20Items)) (Variables|Default|GetLength%20From%20Player)) 0.0 0.0) (+ (.yaw _returnvalue) -9e+01) "0, 0,1.000000") (Transformation|GetActorLocation _player_object_ref)) false false))

(fn GetGamePlayTagContainer
  (return (Variables|Default|GetGamePlay%20Tag%20Container)))

(fn GetMassValue
  (return (Variables|Default|GetMass%20Value)))