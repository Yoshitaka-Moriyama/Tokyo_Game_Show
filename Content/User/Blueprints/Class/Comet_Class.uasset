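; Comet actor that drifts through the game world using a gravity movement component.
; On BeginPlay it caches the main Game Instance, then feeds the GravityMoveComponent an initial 2D push along its yaw, scaled by FloatingSpeed.
; It exposes its gameplay tag container and mass value through getter functions, and has no tick or overlap logic of its own.
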(event EventBeginPlay
  ;[1 1 1] Game Instanceを変数に格納する
  (bind _asmain_game_instance (Utilities|Casting|CastToMainGameInstance (Game|GetGameInstance)))
  (Variables|Default|SetGame%20Instance%20Ref _asmain_game_instance)
  (Default|AddActorPromotion (Variables|Default|GetGravityMoveComponent) (* (Math|Conversions|ToVector2D(Vector) (Class|KismetMathLibrary|CreateVectorfromYawPitch (.yaw (Transformation|GetActorRotation)) 0.0 1.0)) (Variables|Default|GetFloating%20Speed))))

(event Collision|EventActorBeginOverlap
  (params (OtherActor :type Actor%20Object%20Reference)))

(event EventTick
  (params (DeltaSeconds :type Float%20%28single-precision%29)))

(fn ConstructionScript)

(fn GetGamePlayTagContainer
  (return (Variables|Default|GetGamePlay%20Tag%20Container)))

(fn GetMassValue
  (return (Variables|Default|GetMass%20Value)))