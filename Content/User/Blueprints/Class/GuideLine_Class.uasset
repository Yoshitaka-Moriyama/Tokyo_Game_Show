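; GuideLine_Class is a guide-line actor that shows a row of arrows following the player object, indicating its current speed relative to maximum launch speed.
; At BeginPlay it caches the game instance and dynamically spawns the arrow particle components.
; Each Tick derives a clamped arrow count from speed, repositions itself using player yaw, and updates particle color and alpha parameters, graduating blue intensity and hiding surplus arrows.
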(event EventBeginPlay
  (Utilities|FlowControl|DoOnce false
    (:Completed
      ;[1 1 1] Game Instanceを変数に格納する
      (bind _asmain_game_instance (Utilities|Casting|CastToMainGameInstance (Game|GetGameInstance)))
      (Variables|Default|SetGame%20Instance%20Ref _asmain_game_instance)
      (CallFunction|SetArrowComponent))))

(event Collision|EventActorBeginOverlap
  (params (OtherActor :type Actor%20Object%20Reference)))

(event EventTick
  (params (DeltaSeconds :type Float%20%28single-precision%29))
  (CallFunction|SetCurrentArrowCnt)
  (CallFunction|AdjustArrowCnt)
  (CallFunction|SetRelativePosandRot)
  (CallFunction|UpdateMaterial))

(fn ConstructionScript)

(fn SetRelativePosandRot
  (bind _game_instance_ref (Variables|Default|GetGame%20Instance%20Ref))
  (bind _player_object_ref (Variables|/Game/User/Blueprints/Others/MainGameInstance.MainGameInstance_C|GetPlayer%20Object%20Ref _game_instance_ref))
  (bind _returnvalue (Transformation|GetActorRotation _player_object_ref))
  ;[1 1 1] オブジェクトの向きと位置をPlayerObjectに合わせて調整する
  (Transformation|SetActorRotation (Math|Rotator|MakeRotator 0.0 0.0 (+ (.yaw _returnvalue) 1.8e+02)))
  (Transformation|SetActorLocation (+ (Math|Vector|RotateVectorAroundAxis "300.000000, 0, 0" (+ (.yaw _returnvalue) 9e+01) "0, 0,1.000000") (Transformation|GetActorLocation _player_object_ref)) false false))

(fn SetArrowComponent
  ;[1 1 1] Max Arrow Cntの数だけ動的にParticle System Componentを生成し、リストに格納する
  (for _index (range 0 (Variables|Default|GetMax%20Arrow%20Cnt))
    (bind _returnvalue (AddComponent|AddParticleSystemComponent false (Math|Transform|MakeTransform (Math|Vector|MakeVector 0.0 (* _index (* (Variables|Default|GetArrow%20Span) -1.0)) 2e+02) "0.000000,180.000000,0.000000" "3.000000,3.000000,3.000000")))
    (Utilities|Array|Add (Variables|Default|GetParticle%20Comp%20List) _returnvalue)))

(fn UpdateMaterial
  ;[1 1 1] 各矢印のマテリアルに色をセットする
  (for (_array_element _array_index) (Variables|Default|GetParticle%20Comp%20List)
    (Utilities|FlowControl|Sequence
      (:then_0
        (Effects|Components|ParticleSystem|SetVectorParameter _array_element "Color" (.Color (CallFunction|GetColor _array_index))))
      (:then_1
        (Effects|Components|ParticleSystem|SetFloatParameter _array_element "Alpha" (.alpha (CallFunction|GetColor _array_index)))))))

(fn GetColor
  (params (Index :type Integer))
  ;[1 1 1] indexがArrow Cnt以上の場合{0, 0, 0, 0}透明色を、それ以外は｛15, 41, 54, 1｝を返す
  (bind _output_get (LocalVariables|Setmat%20index Index))
  (if (>= _output_get (Variables|Default|GetArrow%20Cnt))
    (return "0, 0, 0" 0.0)
    (else
      (return (* (Math|Vector|MakeVector 0.0 0.0 0.8) (+ (- (Variables|Default|GetMax%20Arrow%20Cnt) (LocalVariables|Getmat%20index)) 1)) 1.0))))

(fn AdjustArrowCnt
  ;[1 1 1] Arrow Cntを0～Max Arrow Cntの範囲に調整する
  (Variables|Default|SetArrow%20Cnt (Math|Integer|Max(Integer) (Variables|Default|GetArrow%20Cnt)))
  (Variables|Default|SetArrow%20Cnt (Math|Integer|Min(Integer) (Variables|Default|GetArrow%20Cnt) (Variables|Default|GetMax%20Arrow%20Cnt))))

(fn SetCurrentArrowCnt
  (bind _game_instance_ref (Variables|Default|GetGame%20Instance%20Ref))
  (bind _player_object_ref (Variables|/Game/User/Blueprints/Others/MainGameInstance.MainGameInstance_C|GetPlayer%20Object%20Ref _game_instance_ref))
  ;[1 1 1] PlayerObjectの速度と最大速度から現在のArrow Cntを設定する
  (Variables|Default|SetArrow%20Cnt (Math|Float|Truncate (/ (* (Variables|Default|GetMax%20Arrow%20Cnt) (Variables|/Game/User/Blueprints/Class/PlayerObject_Class.PlayerObject_Class_C|GetSpeed%20Value _player_object_ref)) (Variables|/Game/User/Blueprints/Class/PlayerObject_Class.PlayerObject_Class_C|GetMax%20Launch%20Speed _player_object_ref)))))

(fn SetVisible
  (params (Flag%20Visible :type Boolean))
  ;[1 1 1] 描画するかどうかを設定する
  (Rendering|SetVisibility (Variables|Default|GetDefaultSceneRoot) Flag%20Visible true)
  (return))