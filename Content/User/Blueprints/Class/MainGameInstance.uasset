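; Game instance that tracks the selected stage in a name list and drives stage switching and reloading.
; Relative changes feed into a direct change, which unloads the current stage, clamps the new index to the list bounds, then loads that stage as visible.
; Loading and unloading go out by level name through dispatcher calls, with the actual level handling left outside these graphs.
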(fn GetCurrentStageName
  (return (Utilities|Array|Get(acopy) (Variables|Default|GetStage%20Name%20List) (Variables|Default|GetStage%20Select%20Index))))

(fn ChangeStageDiff
  (params (Select%20Index%20Diff :type Integer))
  ;[1 1 1] StageをSelect Index Diffの値分だけ変更し、ステージを切り替える
  (CallFunction|ChangeStageDirect (+ Select%20Index%20Diff (Variables|Default|GetStage%20Select%20Index))))

(fn ChangeStageDirect
  (params (Change%20Stage%20Index :type Integer))
  ;[1 1 1] StageをChange Stage Indexの値に変更し、ステージを切り替える
  (Default|CallUnloadLevelDispatcher (CallFunction|GetCurrentStageName))
  (Variables|Default|SetStage%20Select%20Index Change%20Stage%20Index)
  (CallFunction|AdjustStageSelectIndex)
  (Default|CallLoadLevelDispatcher (CallFunction|GetCurrentStageName) true))

(fn AdjustStageSelectIndex
  (bind _stage_name_list (Variables|Default|GetStage%20Name%20List))
  (bind _returnvalue (Utilities|Array|Length _stage_name_list))
  ;[1 1 1] Stage Select Indexを適正な値に調整する
  (if (< (Variables|Default|GetStage%20Select%20Index) 0)
    (Variables|Default|SetStage%20Select%20Index 0))
  (if (>= (Variables|Default|GetStage%20Select%20Index) _returnvalue)
    (Variables|Default|SetStage%20Select%20Index (- _returnvalue 1))))

(fn ReloadCurrentStage
  ;[1 1 1] 現在のステージを再読み込みする
  (Default|CallUnloadLevelDispatcher (CallFunction|GetCurrentStageName))
  (Default|CallLoadLevelDispatcher (CallFunction|GetCurrentStageName) true))