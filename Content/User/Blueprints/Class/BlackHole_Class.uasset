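; Black hole actor that warps actors to a paired white hole, which it spawns at LocationOfWhileHole on BeginPlay while hiding its own mesh.
; Warp deactivates and hides the target, then queues it in WarpActorList with a constant velocity toward the white hole and a distance-based travel time.
; Tick moves queued actors without sweeping, counts down their time, then reactivates, shows and removes them when it expires.
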(event EventBeginPlay
  (|CallParentFunction)
  (Game|SpawnActorfromClass "/Game/User/Blueprints/Class/WhileHole_Class.WhileHole_Class_C" (Math|Transform|MakeTransform (Variables|Default|GetLocationOfWhileHole) "0, 0, 0" "3.000000,3.000000,3.000000") "Undefined" 0 0)
  (Rendering|SetVisibility (Variables|Default|GetStaticMesh) false false))

(event Collision|EventActorBeginOverlap
  (params (OtherActor :type Actor%20Object%20Reference))
  (|CallParentFunction OtherActor))

(event EventTick
  (params (DeltaSeconds :type Float%20%28single-precision%29))
  (CallFunction|UpdateWarpActor DeltaSeconds))

(fn ConstructionScript
  (|CallParentFunction))

(fn UpdateWarpActor
  (params (Delta%20Seconds :type Float%20%28single-precision%29))
  (bind _array_element (Utilities|ForEachLoopRef (Variables|Default|GetWarp%20Actor%20List))
    (:LoopBody
      ;[1 1 1] ワープ速度に従ってアクターを移動させる
      (Utilities|FlowControl|Sequence
        (:then_0
          (Transformation|AddActorWorldOffset (.Actor (Utilities|Struct|BreakWarpActorData _array_element)) (* (.Speed (Utilities|Struct|BreakWarpActorData _array_element)) Delta%20Seconds)))
        (:then_1
          ;[1 1 1] 残り時間を減らす
          (Utilities|Struct|SetmembersinWarpActorData _array_element (- (.RemainTime (Utilities|Struct|BreakWarpActorData _array_element)) Delta%20Seconds)))
        (:then_2
          ;[1 1 1] 残り時間が0になったとき、アクターを有効にしリストから指定のアクターを取り除く
          (if (<= (.RemainTime (Utilities|Struct|BreakWarpActorData _array_element)) 0.0)
            (Class|ActorStateInterface|SetActivation(Message) (.Actor (Utilities|Struct|BreakWarpActorData _array_element)) true true)
            (Utilities|Array|RemoveItem (Variables|Default|GetWarp%20Actor%20List) _array_element)))))))

(fn Warp
  (params (Target%20Actor :type Actor%20Object%20Reference))
  (bind _returnvalue (Transformation|GetActorLocation Target%20Actor))
  (bind _locationofwhilehole (Variables|Default|GetLocationOfWhileHole))
  (bind _returnvalue_2 (- _locationofwhilehole _returnvalue))
  ;[1 1 1] ワープさせるための情報を計算し、ワープリストに格納する
  (Class|ActorStateInterface|SetActivation(Message) Target%20Actor false false)
  (Utilities|Array|Add (Variables|Default|GetWarp%20Actor%20List) (Utilities|Struct|MakeWarpActorData Target%20Actor (* (Math|Vector|Normalize _returnvalue_2) (Variables|Default|GetWarp%20Speed)) (/ (Math|Vector|VectorLength _returnvalue_2) (Variables|Default|GetWarp%20Speed))))
  (return true))