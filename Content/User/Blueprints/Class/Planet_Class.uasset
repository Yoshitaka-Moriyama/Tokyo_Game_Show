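; Planet actor that acts as a 2D gravity source and exposes its gameplay tag container.
; On BeginPlay it spawns a colored ring particle scaled to the gravity range, then destroys it on EndPlay.
; GetGravityEffect returns a pull toward the planet from both masses, divided by either linear distance or a fixed length, times a tuning ratio.
; The range check is disconnected, so the pull is not cut off outside the ring.
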(event EventBeginPlay
  ;[1 1 1] 重力範囲を示すパーティクルを発生させる
  (bind _returnvalue (Effects|SpawnEmitteratLocation "/Game/User/Particle/GravityEffectRing_Particle.GravityEffectRing_Particle" (Transformation|GetActorLocation) "0, 0, 0" (* "1.000000,1.000000,1.000000" (* (/ (Variables|Default|GetGravity%20Effect%20Length) 1e+02) 2.0)) false))
  (bind _output_get (Variables|Default|SetGravity%20Aera%20Particle _returnvalue))
  (Effects|Components|ParticleSystem|SetVectorParameter _output_get "Color" "50.000000,20.000000,10.000000"))

(event Collision|EventActorBeginOverlap
  (params (OtherActor :type Actor%20Object%20Reference)))

(event EventEndPlay
  (params (EndPlayReason :type EEndPlayReason%20Enum :default "Destroyed"))
  (Components|DestroyComponent (Variables|Default|GetGravity%20Aera%20Particle)))

(fn ConstructionScript)

(fn GetGamePlayTagContainer
  (return (Variables|Default|GetGamePlay%20Tag%20Container)))

(fn GetGravityEffect
  (params (Mass%20Effected :type Float%20%28single-precision%29) (Pos%20Effected :type Vector%202D%20Structure))
  (bind _returnvalue (Transformation|GetActorLocation))
  (bind _returnvalue_2 (Math|Conversions|ToVector2D(Vector) _returnvalue))
  (bind _returnvalue_3 (- _returnvalue_2 Pos%20Effected))
  ;[1 1 1] 重力効果を計算し返す関数
  (if false
    (return "")
    (else
      (return (* (Math|Vector2D|Normalize2D _returnvalue_3) (* (/ (* Mass%20Effected (Variables|Default|GetMass%20Value)) (Math|Float|SelectFloat (Math|Vector2D|Vector2DLength _returnvalue_3) 3e+03 (Variables|Default|GetFlag%20Depend%20On%20Length))) (Variables|Default|GetSpeed2Gravity%20Ratio)))))))